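; Test homing missile that launches along its mesh's forward vector and keeps turning to face a DebugTarget actor found at BeginPlay.
; BeginPlay sets a one-time physics velocity and activates the thruster effect.
; Each Tick snaps rotation to the target with physics teleport, sets angular velocity from the look-at direction vector, and prints current speed.
; Tick never redirects linear velocity, and a velocity clamp node sits unused.
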(event EventBeginPlay
  (bind _returnvalue (Actor|GetActorOfClass "/Game/DebugTarget.DebugTarget_C"))
  (Variables|Default|SetTarget _returnvalue)
  (Physics|SetPhysicsLinearVelocity (Variables|Character|GetMesh) (* (Math|Vector|GetForwardVector (Variables|Character|GetMesh)) (Variables|Default|GetInitial%20Vel)) false "None")
  (Components|Activation|SetActive (Variables|Default|GetThrusterFX) true true))

(event EventTick
  (params (DeltaSeconds :type Float%20%28single-precision%29))
  (bind _returnvalue (Transformation|GetActorLocation))
  (bind _target (Variables|Default|GetTarget))
  (bind _mesh (Variables|Character|GetMesh))
  (bind _returnvalue_2 (Transformation|GetActorLocation _target))
  (bind _returnvalue_3 (Math|Rotator|FindLookatRotation _returnvalue _returnvalue_2))
  (bind _returnvalue_4 (Physics|GetPhysicsLinearVelocity _mesh "None"))
  (Transformation|SetActorRotation _returnvalue_3 true)
  (Class|PrimitiveComponent|SetPhysicsAngularVelocityinDegrees _mesh (Math|Rotator|GetRotationXVector _returnvalue_3) false "None")
  (Development|PrintString (Utilities|String|ToString(Float) (Math|Vector|VectorLength _returnvalue_4))))

(fn ConstructionScript)