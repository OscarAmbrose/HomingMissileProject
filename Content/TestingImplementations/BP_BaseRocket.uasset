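; Base test rocket actor, assembled from data-driven component slots, that flies toward a target and explodes on capsule overlap.
; BeginPlay feeds each slot's stats into StatManager and adds its component class, or failing that a socket-attached mesh.
; After a short delay, Tick launches RocketMovement once and keeps updating its target; engine shutoff destroys the thruster FX.
; Explosion spawns sound and an emitter scaled by Destructivity, then destroys the actor.
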(event OnEngineDisabled(RocketMovement)
  (Components|DestroyComponent (Variables|Default|GetThrusterFX)))

(event OnComponentBeginOverlap(Capsule)
  (params (OverlappedComponent :type Primitive%20Component%20Object%20Reference) (OtherActor :type Actor%20Object%20Reference) (OtherComp :type Primitive%20Component%20Object%20Reference) (OtherBodyIndex :type Integer) (bFromSweep :type Boolean) (SweepResult :type Hit%20Result%20Structure%20%28by%20ref%29))
  (Class|BaseRocket|ExplodeRocket))

(event EventBeginPlay
  (CallFunction|SetupStats)
  (Utilities|FlowControl|Delay 0.5)
  (Components|Activation|SetActive (Variables|Default|GetThrusterFX) true true)
  (Actor|Tick|SetActorTickEnabled true))

(event EventTick
  (params (DeltaSeconds :type Float%20%28single-precision%29))
  (bind _rocketmovement (Variables|Default|GetRocketMovement))
  (bind _currenttargetlocation (Variables|Default|GetCurrentTargetLocation))
  ;[0.15 0.15 0.15 0.5] There are much better ways to do this
  (Variables|/Script/HomingMissileProject.RocketMovement|SetTargetLocation _rocketmovement _currenttargetlocation)
  (Utilities|FlowControl|DoOnce false
    (:Completed
      (Class|RocketMovement|StartRocketwithVelocity _rocketmovement (* (Math|Vector|Normalize (- _currenttargetlocation (Transformation|GetActorLocation))) (Variables|Default|GetLaunchSpeed))))))

(event EventExplodeRocket
  (bind _returnvalue (Transformation|GetActorLocation))
  (bind _returnvalue_2 (Transformation|GetActorForwardVector))
  (bind _statmanager (Variables|Default|GetStatManager))
  (bind (_foundvalue _success) (Class|RocketStatManager|GetStat _statmanager "Destructivity"))
  (bind _returnvalue_3 (* _returnvalue_2 2e+02))
  (bind _returnvalue_4 (+ _returnvalue _returnvalue_3))
  (Effects|SpawnEmitteratLocation "/Game/Realistic_Starter_VFX_Pack_Vol2/Particles/Explosion/P_Explosion_Big_B.P_Explosion_Big_B" _returnvalue_4 "0, 0, 0" (Math|Vector|SelectVector (Math|Vector|ClampVectorSize (Math|Vector|Lerp(Vector) "1.000000,1.000000,1.000000" "5.000000,5.000000,5.000000" (/ _foundvalue 2e+02)) 1.0 8.9) "1.000000,1.000000,1.000000" _success))
  (Audio|PlaySoundatLocation "/Engine/EditorSounds/GamePreview/PossessPlayer_Cue.PossessPlayer_Cue" _returnvalue_4 "0, 0, 0" 1.0 1.0 0.0 0 0 0 0)
  (Actor|DestroyActor))

(event Collision|EventActorBeginOverlap
  (params (OtherActor :type Actor%20Object%20Reference)))

(fn ConstructionScript)

(fn SetupStats
  ;[0.15 0.15 0.15 0.5] This should not exist - the temporary becomes permanent with a deadline
  (for _array_element (Variables|Default|GetComponentSlots)
    (Utilities|IsValid (.ComponentData (Utilities|Struct|BreakMissileComponentSlot _array_element))
      (:Is%20Valid
        (bind (_keypin _valuepin) (Utilities|Map|ForEachLoop(Map) (Variables|/Script/HomingMissileProject.RocketComponentDataBase|GetStatMap (.ComponentData (Utilities|Struct|BreakMissileComponentSlot _array_element))))
          (:then
            (Class|RocketStatManager|ModifyStat (Variables|Default|GetStatManager) _keypin _valuepin))
          (:CompletedPin
            (if (Utilities|IsValidClass (Variables|/Script/HomingMissileProject.RocketComponentDataBase|GetComponentToAdd (.ComponentData (Utilities|Struct|BreakMissileComponentSlot _array_element))))
              (Game|AddComponentbyClass (Variables|/Script/HomingMissileProject.RocketComponentDataBase|GetComponentToAdd (.ComponentData (Utilities|Struct|BreakMissileComponentSlot _array_element))))
              (else
                (Utilities|IsValid (Variables|/Script/HomingMissileProject.RocketComponentDataBase|GetStaticMesh (.ComponentData (Utilities|Struct|BreakMissileComponentSlot _array_element)))
                  (:Is%20Valid
                    (bind _returnvalue (Game|AddComponentbyClass "/Script/Engine.StaticMeshComponent" false (Math|Transform|MakeTransform "0, 0, 0" "90.000000,0.000000,0.000000" "0.300000,0.300000,1.000000")))
                    (Components|StaticMesh|SetStaticMesh _returnvalue (Variables|/Script/HomingMissileProject.RocketComponentDataBase|GetStaticMesh (.ComponentData (Utilities|Struct|BreakMissileComponentSlot _array_element))))
                    (Transformation|AttachComponentToComponent _returnvalue (Variables|Default|GetSkeletalMesh) (Variables|/Script/HomingMissileProject.RocketComponentDataBase|GetSocketToAttachTo (.ComponentData (Utilities|Struct|BreakMissileComponentSlot _array_element))) "SnapToTarget" "KeepRelative" "KeepRelative" true)))))))))))